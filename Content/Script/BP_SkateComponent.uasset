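; BP_SkateComponent is a hover component that suspends a physics-simulated primitive, apparently a skateboard, above surfaces.
; InitComponent stores the supplied mesh and enables its physics.
; Each CustomEvent call traces world-down from the component and pushes the mesh along the impact normal, with force fading linearly over the trace length.
; The branch is hardwired true, so force and fixed linear and angular damping apply without a hit check.
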(event `InitComponent`
  (params (MeshComponent :type "SkeletalMeshComponent Object Reference"))
  (bind _asprimitive_component (cast `PrimitiveComponent` MeshComponent))
  (bind _output_get (set `self.ParentComponentSkate` _asprimitive_component))
  (`PrimitiveComponent.SetSimulatePhysics` _output_get true))

(event `CustomEvent`
  (params (DeltaSeconds :type "Float (single-precision)"))
  (bind _returnvalue (`self.K2_GetComponentLocation`))
  (bind _parentcomponentskate (`self.ParentComponentSkate`))
  (bind _outhit (`KismetSystemLibrary.LineTraceSingle` _returnvalue (+ (* (`KismetMathLibrary.GetUpVector` (struct)) (* (`self.TraceLength`) -1.0)) _returnvalue) "TraceTypeQuery1"))
  (if true
    (bind (_bblockinghit _binitialoverlap _time _distance _location _impactpoint _normal _impactnormal) (`GameplayStatics.BreakHitResult` _outhit))
    (`PrimitiveComponent.AddForceAtLocation` _parentcomponentskate (* _impactnormal (`KismetMathLibrary.Lerp` (`self.HoverForce`) 0.0 (/ (`KismetMathLibrary.VSize` (- _location (`self.K2_GetComponentLocation`))) (`self.TraceLength`)))) (`self.K2_GetComponentLocation`) "None")
    (`PrimitiveComponent.SetLinearDamping` _parentcomponentskate 3.0)
    (`PrimitiveComponent.SetAngularDamping` _parentcomponentskate 5.0)))